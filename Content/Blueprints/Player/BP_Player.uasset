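; Player Blueprint with a top-down spring-arm camera and input-driven movement states.
; Holding the middle mouse button enables clamped pitch adjustment, while the scroll wheel sets clamped boom length; both feed CameraUpdate, which also applies lag settings and runs at construction.
; Right mouse switches to aiming and Left Ctrl to walking, each returning to running on release.
; A CameraShake function plays a world shake at the camera's location.
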(event `Key|MiddleMouseButton`
  (params (Key :type "Key Structure"))
  ;[0 0 0 1 32] Camera control
  ;;[0 0 0] Press the mouse wheel to control camera rotation
  (:`Pressed`
    (set `self.IsMovingCamera` true))
  (:`Released`
    (set `self.IsMovingCamera` false)))

(event `InputAxis|LookUp`
  (params (AxisValue :type "Float (single-precision)"))
  (bind (_rotation_roll _rotation_pitch _rotation_yaw) (`KismetMathLibrary.BreakRotator` (`self.Rotation`)))
  ;[0 0 0 1 32] Camera control
  ;;[0 0 0] Press the mouse wheel to control camera rotation
  (if (`self.IsMovingCamera`)
    (set `self.Rotation` (`KismetMathLibrary.MakeRotator` _rotation_roll (`KismetMathLibrary.FClamp` (+ _rotation_pitch (* AxisValue 5.0)) -90.0 -45.0) _rotation_yaw))
    (`self.CameraUpdate`)))

(event `Key|RightMouseButton`
  (params (Key :type "Key Structure"))
  (:`Pressed`
    (`self.ChangeMovementState` "Aim_State"))
  (:`Released`
    (`self.ChangeMovementState` "Run_State")))

(event `InputAxisKey|MouseWheelAxis`
  (params (AxisValue :type "Float (single-precision)"))
  ;[0 0 0 1 32] Camera control
  ;;[0 0 0] Scroll the mouse wheel to control the height of the camera
  (set `self.Height` (`KismetMathLibrary.FClamp` (+ (* AxisValue -50.0) (`self.Height`)) 700.0 2000.0))
  (`self.CameraUpdate`))

(event `Key|LeftControl`
  (params (Key :type "Key Structure"))
  (:`Pressed`
    (`self.ChangeMovementState` "Walk_State"))
  (:`Released`
    (`self.ChangeMovementState` "Run_State")))

(fn `CameraShake`
  (`GameplayStatics.PlayWorldCameraShake` "/Game/Blueprints/Player/BP_CameraShake.BP_CameraShake_C" (`SceneComponent.K2_GetComponentLocation` (`self.TopDownCameraComponent`)) 0.0 30.0))

(fn `CameraUpdate`
  (bind _cameraboom (`self.CameraBoom`))
  (set `SpringArmComponent.TargetArmLength` (`self.Height`) _cameraboom)
  (`SceneComponent.K2_SetRelativeRotation` _cameraboom (`self.Rotation`) false false)
  (set `SpringArmComponent.bEnableCameraLag` (`self.Flow`) _cameraboom)
  (set `SpringArmComponent.CameraLagSpeed` (`self.Camera speed`) _cameraboom))

(fn `UserConstructionScript`
  (`self.CameraUpdate`))